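; BP_PlayerHUD is a HUD Blueprint that draws a small dot crosshair at screen center while the player aims.
; Each DrawHUD pass casts the player pawn to BP_Character, does nothing if the cast fails, and checks its Aiming flag.
; The dot is two stacked DrawRect calls, a black square behind a smaller white one, giving it a dark outline.
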(event `self.ReceiveDrawHUD`
  (params (SizeX :type Integer) (SizeY :type Integer))
  (bind _returnvalue (`KismetMathLibrary.Conv_IntToDouble` (/ SizeX 2)))
  (bind _returnvalue_2 (`KismetMathLibrary.Conv_IntToDouble` (/ SizeY 2)))
  (bind _asbp_character (cast `/Game/Blueprints/Characters/BP_Character` (`GameplayStatics.GetPlayerPawn` 0)))
  (if (`/Game/Blueprints/Characters/BP_Character.Aiming` _asbp_character)
    (`self.DrawRect` (struct :`A` 1.0) (- _returnvalue 1.0) (- _returnvalue_2 1.0) 4.0 4.0)
    (`self.DrawRect` (struct :`R` 1.0 :`G` 1.0 :`B` 1.0 :`A` 1.0) _returnvalue _returnvalue_2 2.0 2.0)))

(fn `UserConstructionScript`)