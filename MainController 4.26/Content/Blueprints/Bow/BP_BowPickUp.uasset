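; BP_BowPickUp is a pickup that gives the bow to the player character on overlap.
; On BeginPlay it disables collision on every actor tagged "Aimer".
; When a BP_Character overlaps it, it sets HasBow, calls GiveBow and destroys itself, then unhides the "Aimer" actors and enables their collision.
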(event `self.ReceiveBeginPlay`
  (bind _outactors (`GameplayStatics.GetAllActorsWithTag` "Aimer"))
  (for _array_element _outactors
    (`self.SetActorEnableCollision` _array_element false)))

(event `self.ReceiveActorBeginOverlap`
  (params (OtherActor :type "Actor Object Reference"))
  (bind _asbp_character (cast `/Game/Blueprints/Characters/BP_Character` OtherActor))
  (set `/Game/Blueprints/Characters/BP_Character.HasBow` true _asbp_character)
  (`/Game/Blueprints/Characters/BP_Character.GiveBow` _asbp_character)
  (`self.K2_DestroyActor`)
  (bind _outactors (`GameplayStatics.GetAllActorsWithTag` "Aimer"))
  (for _array_element _outactors
    (`self.SetActorHiddenInGame` _array_element false)
    (`self.SetActorEnableCollision` _array_element true)))

(fn `UserConstructionScript`)