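; Master bow actor for BP_Character that handles aiming visuals, drawing and shooting of normal and teleport arrows.
; Normal arrows use a fixed-damage camera sphere trace with a cosmetic tracer, timing surface-based impact effects to its flight.
; Teleport arrows spawn real projectiles, with speed and damage scaled by a draw timeline.
; Damage handling adds radial impulse and leaves arrow pickups on non-physics surfaces, attached and non-collectable on bone hits.
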(event `BeginPlayBow`
  (params (Character :type "Object Object Reference"))
  ;[1 1 1] BeginPlay
  (bind _asbp_character (cast `/Game/Blueprints/Characters/BP_Character` Character))
  (`self.SetOwner` _asbp_character)
  (set `self.CharacterReference` _asbp_character)
  (`self.DontHoldCable`))

(event `self.ReceiveTick`
  (params (DeltaSeconds :type "Float (single-precision)"))
  (bind _arrowmesh (`self.ArrowMesh`))
  ;[0.5558 1 0.5477] EventTick
  (set `self.ArrowType` (`/Game/Blueprints/Characters/BP_Character.ArrowType` (`self.CharacterReference`)))
  (if (`self.IsAimingAndNotShootingHasAmmo`)
    (`SceneComponent.SetHiddenInGame` _arrowmesh false false)
    (`self.SetArrowLocationAndRotation` DeltaSeconds)
    (`self.AttachArrowToHand`)
    (`/Game/Blueprints/Characters/BP_Character.Add Arrows` (`self.CharacterReference`) 0 0)
    (else
      (`SceneComponent.SetHiddenInGame` _arrowmesh true false))))

(event `HoldCable`
  ;[1 1 1] Hold or Dont Hold the Cable
  (`CableComponent.SetAttachEndTo` (`self.BottomCable`) (`self.CharacterReference`) "Mesh" "Bip001_Middle1_R")
  (`CableComponent.SetAttachEndTo` (`self.TopCable`) (`self.CharacterReference`) "Mesh" "Bip001_Middle1_R"))

(event `DontHoldCable`
  ;[1 1 1] Hold or Dont Hold the Cable
  (`CableComponent.SetAttachEndTo` (`self.BottomCable`) null "Bow" "BowIdle")
  (`CableComponent.SetAttachEndTo` (`self.TopCable`) null "Bow" "BowIdle")
  (`SceneComponent.K2_AttachToComponent` (`self.ArrowScene`) (`self.Bow`) "BowIdle" "SnapToTarget" "KeepRelative" "KeepWorld" true))

(event `Shoot`
  ;[1 1 1] ShootingEvent
  (switch `/Game/Blueprints/Bow/EnumAmmoType` (`self.ArrowType`)
    (:`NewEnumerator0`
      (set `self.Damage` 100.0)
      (set `self.ShootingDistance` 4000.0)
      (bind _outhit (`self.SphereTraceShot`))
      (`self.TraceSpawnProjectile` (`self.Damage`) _outhit))
    (:`NewEnumerator1`
      (bind _spawntransform (`self.CalculateProjectileInfo`))
      (`self.SpawnProjectile` _spawntransform)
      (`self.Stop DrawTimeline`))))

(event `Fire Effects`
  ;[1 1 1] FireEffects
  (`GameplayStatics.PlaySoundAtLocation` (`self.ShootSound`) (`SceneComponent.K2_GetComponentLocation` (`self.Bow`)) (struct) 1.0 1.0 0.0 null null null)
  (`GameplayStatics.SpawnEmitterAtLocation` (`self.Fire Particle`) (`SceneComponent.K2_GetComponentLocation` (`self.DrawSound`))))

(event `PlayImpactParticle`
  (params (Hit :type "HitResult Structure"))
  ;[1 1 1] ImpactSoundAndParticle
  (`self.PlayImpactParticleAtLocation` Hit))

(event `PlayImpactSound`
  (params (NewParam :type "HitResult Structure"))
  ;[1 1 1] ImpactSoundAndParticle
  (`self.PlayImpactSoundAtLocation` NewParam))

(event `DamageEvent`
  (params (Hitresults :type "HitResult Structure") (BaseDamage :type "Float (double-precision)") (IsSpecialArrow :type Boolean))
  (bind (_bblockinghit _binitialoverlap _time _distance _location _impactpoint _normal _impactnormal _physmat _hitactor) (`GameplayStatics.BreakHitResult` Hitresults))
  (bind (_bblockinghit_2 _binitialoverlap_2 _time_2 _distance_2 _location_2 _impactpoint_2 _normal_2 _impactnormal_2 _physmat_2 _hitactor_2 _hitcomponent) (`GameplayStatics.BreakHitResult` (`self.HitVariable`)))
  (bind (_bblockinghit_3 _binitialoverlap_3 _time_3 _distance_3 _location_3 _impactpoint_3 _normal_3 _impactnormal_3 _physmat_3 _hitactor_3 _hitcomponent_2 _hitbonename) (`GameplayStatics.BreakHitResult` (`self.HitVariable`)))
  (bind _returnvalue (`Pawn.GetController` (`self.CharacterReference`)))
  (bind _returnvalue_2 (== _hitbonename "None"))
  (bind (_returnvalue_roll _returnvalue_pitch _returnvalue_yaw) (`KismetMathLibrary.BreakRotator` (`KismetMathLibrary.FindLookAtRotation` (`SceneComponent.K2_GetComponentLocation` (`Character.Mesh` (`self.CharacterReference`))) (+ _location_2 _normal_2))))
  (bind _returnvalue_3 (+ _returnvalue_roll 90.0))
  (bind _returnvalue_4 (+ _returnvalue_pitch -40.0 (`KismetMathLibrary.RandomFloatInRange` 0.0 30.0)))
  ;[1 1 1] Damage and spawning of shot arrows
  (bind _output_get (set `self.HitVariable` Hitresults))
  (if _bblockinghit
    (`GameplayStatics.ApplyPointDamage` _hitactor BaseDamage (`SceneComponent.K2_GetComponentLocation` (`self.Bow`)) _output_get _returnvalue _returnvalue)
    (`/Engine/EditorBlueprintResources/StandardMacros.IsValid` _hitcomponent
      (:`Is Valid`
        (`PrimitiveComponent.AddRadialImpulse` _hitcomponent _impactpoint_2 500.0 50000.0 "RIF_Constant" false))
      (:`Is Not Valid`
        _))
    (if (`SceneComponent.IsAnySimulatingPhysics` _hitcomponent)
      _
      (elif IsSpecialArrow
        (bind _returnvalue_5 (`|SpawnActorFromClass` "/Game/Blueprints/Bow/BP_Special_Arrow_Pickup.BP_Special_Arrow_Pickup_C" (`KismetMathLibrary.MakeTransform` _impactpoint_2 (`KismetMathLibrary.MakeRotator` _returnvalue_3 _returnvalue_4 _returnvalue_yaw)) "AlwaysSpawn" "OverrideRootScale" null 1 null))
        (if (not _returnvalue_2)
          (`/Engine/EditorBlueprintResources/StandardMacros.IsValid` _hitcomponent_2
            (:`Is Valid`
              (`/Engine/EditorBlueprintResources/StandardMacros.IsValid` _returnvalue_5
                (:`Is Valid`
                  (`self.K2_AttachToComponent` _returnvalue_5 _hitcomponent_2 _hitbonename "SnapToTarget" "KeepWorld" "KeepWorld" true)
                  (set `/Game/Blueprints/Bow/BP_Special_Arrow_Pickup.CanPickUp` false _returnvalue_5))))))
        (else
          (bind _returnvalue_6 (`|SpawnActorFromClass` "/Game/Blueprints/Bow/BP_Arrow_Pickup.BP_Arrow_Pickup_C" (`KismetMathLibrary.MakeTransform` _impactpoint_2 (`KismetMathLibrary.MakeRotator` _returnvalue_3 _returnvalue_4 _returnvalue_yaw)) "AlwaysSpawn" "OverrideRootScale" null 1 null))
          (if (not _returnvalue_2)
            (`/Engine/EditorBlueprintResources/StandardMacros.IsValid` _hitcomponent_2
              (:`Is Valid`
                (`/Engine/EditorBlueprintResources/StandardMacros.IsValid` _returnvalue_6
                  (:`Is Valid`
                    (`self.K2_AttachToComponent` _returnvalue_6 _hitcomponent_2 _hitbonename "SnapToTarget" "KeepWorld" "KeepWorld" true)
                    (set `/Game/Blueprints/Bow/BP_Arrow_Pickup.CanPickUp` false _returnvalue_6)))))))))))

(event `StartDrawTimeline`
  (params (DamageSettingsPlayRate :type "Float (double-precision)"))
  ;[1 1 1] StartDrawingAndSetVariables
  (`AudioComponent.Play` (`self.DrawSound`) 0.0)
  (`TimelineComponent.SetPlayRate` (`self.DamageSettings`) DamageSettingsPlayRate)
  (bind (_direction _lerplinear) (`Timeline|DamageSettings` :!label _label)
    (:`Update`
      (if (not (`|EnumEquality` (`self.ArrowType`) "NewEnumerator0"))
        (bind _output_get (set `self.DrawPercentage` _lerplinear))
        (set `self.Damage` (`KismetMathLibrary.Lerp` (`self.DamageMin`) (`self.DamageMax`) _output_get))
        (set `self.ShootingDistance` (`KismetMathLibrary.Lerp` (`self.ShootingDistanceMin`) (`self.ShootingDistanceMax`) _output_get))
        (set `self.ProjectileSpeed` (`KismetMathLibrary.Lerp` (`self.ProjectileSpeedMin`) (`self.ProjectileSpeedMax`) _output_get))))
    (:`Finished`
      (`AudioComponent.FadeOut` (`self.DrawSound`) 0.2 0.0 "Linear"))))

(event `ReverseDrawTimeline`
  (params (DamageSettingsPlayRate :type "Float (double-precision)"))
  ;[1 1 1] StartDrawingAndSetVariables
  (goto _label :!via `Reverse`))

(event `Stop DrawTimeline`
  ;[1 1 1] StartDrawingAndSetVariables
  (`|ExecutionSequence`
    (:`then_0`
      (goto _label :!via `Stop`))
    (:`then_1`
      (goto _label :!via `SetNewTime`))
    (:`then_2`
      (set `self.DrawPercentage` 0.0)
      (set `self.ProjectileSpeed` (`self.ProjectileSpeedMin`))
      (set `self.ShootingDistance` (`self.ShootingDistanceMin`))
      (set `self.Damage` (`self.DamageMin`)))))

(fn `AttachArrowToHand`
  (`SceneComponent.K2_AttachToComponent` (`self.ArrowScene`) (`Character.Mesh` (`self.CharacterReference`)) "Bip001_Hand_R" "SnapToTarget" "KeepRelative" "KeepWorld" true))

(fn `CalculateProjectileInfo`
  (returns (SpawnTransform :type "Transform Structure"))
  (bind _characterreference (`self.CharacterReference`))
  (bind _returnvalue (`SceneComponent.K2_GetComponentLocation` (`self.ArrowSpawnLocation`)))
  (bind _camera (`/Game/Blueprints/Characters/BP_Character.Camera` _characterreference))
  (bind _returnvalue_2 (`SceneComponent.K2_GetComponentLocation` _camera))
  (bind _returnvalue_3 (`SceneComponent.GetForwardVector` _camera))
  (bind _returnvalue_4 (+ _returnvalue_2 (* (`KismetMathLibrary.RandomUnitVectorInConeInDegrees` _returnvalue_3 1.0) (`KismetMathLibrary.FClamp` (`self.ProjectileSpeed`) 0.0 60000.0))))
  (bind (_outhit _returnvalue_5) (`KismetSystemLibrary.SphereTraceSingle` (+ _returnvalue_2 (* _returnvalue_3 (`self.ArrowStartLocationOffset`))) _returnvalue_4 (`self.TraceRadius`) "TraceTypeQuery1" false (`|MakeArray` _characterreference :!type "Actor Object Reference")))
  (if _returnvalue_5
    (return (`KismetMathLibrary.MakeTransform` _returnvalue (`KismetMathLibrary.FindLookAtRotation` _returnvalue (`.ImpactPoint` (`GameplayStatics.BreakHitResult` _outhit)))))
    (else
      (return (`KismetMathLibrary.MakeTransform` _returnvalue (`KismetMathLibrary.FindLookAtRotation` _returnvalue _returnvalue_4))))))

(fn `IsAimingAndNotShootingHasAmmo`
  (returns (ReturnValue :type Boolean))
  (switch `/Game/Blueprints/Bow/EnumAmmoType` (`self.ArrowType`)
    (:`NewEnumerator0`
      (return (and (`self.IsAiming`) (not (`self.Shooting`)) (not (`self.OutOfAmmo`)))))
    (:`NewEnumerator1`
      (return (and (`self.IsAiming`) (not (`self.Shooting`)) (not (`self.OutOfTeleportAmmo`)))))))

(fn `PlayImpactParticleAtLocation`
  (params (Hit :type "HitResult Structure (by ref)"))
  (bind (_bblockinghit _binitialoverlap _time _distance _location _impactpoint _normal _impactnormal _physmat _hitactor _hitcomponent _hitbonename _hititem _faceindex _tracestart _traceend) (`GameplayStatics.BreakHitResult` Hit))
  (bind _brick_impact_effect (`self.Brick_Impact_Effect`))
  (bind _returnvalue (select `bool` _bblockinghit :`false` _traceend :`true` _impactpoint))
  (bind _returnvalue_2 (select `EPhysicalSurface` (`PhysicalMaterial.SurfaceType` _physmat) :`SurfaceType_Default` _brick_impact_effect :`SurfaceType1` _brick_impact_effect :`SurfaceType2` (`self.Dirt_Impact_Effect`) :`SurfaceType3` (`self.Wood_Impact_Effect`) :`SurfaceType4` (`self.Blood_Impact_Effect`) :`SurfaceType5` (`self.Water_Impact_Effect`)))
  (if _bblockinghit
    (`/Engine/EditorBlueprintResources/StandardMacros.IsValid` _returnvalue_2
      (:`Is Valid`
        (`GameplayStatics.SpawnEmitterAtLocation` _returnvalue_2 _returnvalue (struct) (0.3 0.3 0.3)))
      (:`Is Not Valid`
        (`GameplayStatics.SpawnEmitterAtLocation` (`self.Default_Impact_Effect`) _returnvalue (struct) (0.2 0.2 0.2))))))

(fn `PlayImpactSoundAtLocation`
  (params (Hit :type "HitResult Structure (by ref)"))
  (bind (_bblockinghit _binitialoverlap _time _distance _location _impactpoint _normal _impactnormal _physmat) (`GameplayStatics.BreakHitResult` Hit))
  (bind _default_impact_sound (`self.Default_Impact_Sound`))
  (bind _returnvalue (select `EPhysicalSurface` (`PhysicalMaterial.SurfaceType` _physmat) :`SurfaceType_Default` _default_impact_sound :`SurfaceType1` (`self.Brick_Impact_Sound`) :`SurfaceType2` (`self.Dirt_Impact_Sound`) :`SurfaceType3` (`self.Wood_Impact_Sound`) :`SurfaceType4` (`self.Blood_Impact_Sound`) :`SurfaceType5` (`self.Water_Impact_Sound`)))
  (if _bblockinghit
    (`/Engine/EditorBlueprintResources/StandardMacros.IsValid` _returnvalue
      (:`Is Valid`
        (`GameplayStatics.PlaySoundAtLocation` _returnvalue _impactpoint (struct) 1.0 1.0 0.0 null null null))
      (:`Is Not Valid`
        (`GameplayStatics.PlaySoundAtLocation` _default_impact_sound _impactpoint (struct) 1.0 1.0 0.0 null null null)))))

(fn `SetArrowLocationAndRotation`
  (params (DeltaTime :type "Float (double-precision)"))
  (returns (ReturnValue :type "Rotator Structure"))
  (bind _arrowscene (`self.ArrowScene`))
  (bind (_returnvalue_x _returnvalue_y _returnvalue_z) (`KismetMathLibrary.BreakVector` (`SceneComponent.K2_GetComponentLocation` (`self.Bow`))))
  (bind _returnvalue (`KismetMathLibrary.RInterpTo` (`SceneComponent.K2_GetComponentRotation` _arrowscene) (`KismetMathLibrary.FindLookAtRotation` (`SceneComponent.K2_GetComponentLocation` (`self.ArrowScene`)) (`KismetMathLibrary.MakeVector` _returnvalue_x _returnvalue_y _returnvalue_z)) DeltaTime 50.0))
  (`SceneComponent.K2_SetWorldRotation` _arrowscene _returnvalue false false)
  (return _returnvalue))

(fn `SetShootingVariables`
  (params (DrawPercentage :type "Float (double-precision)"))
  (switch `/Game/Blueprints/Bow/EnumAmmoType` (`self.ArrowType`)
    (:`NewEnumerator0`
      (set `self.Damage` 100.0)
      (set `self.ShootingDistance` 4000.0)
      (return))
    (:`NewEnumerator1`
      (bind _output_get (set `self.DrawPercentage` DrawPercentage))
      (set `self.Damage` (`KismetMathLibrary.Lerp` (`self.DamageMin`) (`self.DamageMax`) _output_get))
      (set `self.ShootingDistance` (`KismetMathLibrary.Lerp` (`self.ShootingDistanceMin`) (`self.ShootingDistanceMax`) _output_get))
      (set `self.ProjectileSpeed` (`KismetMathLibrary.Lerp` (`self.ProjectileSpeedMin`) (`self.ProjectileSpeedMax`) _output_get)))))

(fn `SphereTraceShot`
  (returns (OutHit :type "HitResult Structure"))
  (bind _camera (`/Game/Blueprints/Characters/BP_Character.Camera` (`self.CharacterReference`)))
  (bind _returnvalue (`SceneComponent.K2_GetComponentLocation` _camera))
  (bind _returnvalue_2 (`SceneComponent.GetForwardVector` _camera))
  (bind _outhit (`KismetSystemLibrary.SphereTraceSingle` (+ _returnvalue (* _returnvalue_2 (`self.ArrowStartLocationOffset`))) (+ _returnvalue (* (`KismetMathLibrary.RandomUnitVectorInConeInDegrees` _returnvalue_2 (`self.TraceSpread`)) (`self.ShootingDistance`))) (`self.TraceRadius`) "TraceTypeQuery1"))
  (return _outhit))

(fn `UserConstructionScript`)