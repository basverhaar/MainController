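; Master bow projectile that flies at a configurable speed and reports special-arrow damage on impact.
; It follows its velocity, activates particles shortly after spawn and applies its gravity scale after a configurable delay.
; Hitting the bow's own character destroys it.
; Other hits repeat a sphere trace with a growing radius until it finds a result, which goes to the bow's DamageEvent before the projectile destroys itself.
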(event `self.ReceiveBeginPlay`
  (`|ExecutionSequence`
    (:`then_0`
      (`KismetSystemLibrary.Delay` 0.05)
      (`ActorComponent.Activate` (`self.ParticleSystem`) false))
    (:`then_1`
      (`self.SetActorTickEnabled` true)
      (set `ProjectileMovementComponent.bRotationFollowsVelocity` true (`self.ProjectileMovement`))
      (`KismetSystemLibrary.Delay` (`self.DelayBeforeGravity`))
      (set `ProjectileMovementComponent.ProjectileGravityScale` (`self.GravityScale`) (`self.ProjectileMovement`)))))

(event `self.ReceiveTick`
  (params (DeltaSeconds :type "Float (single-precision)"))
  (`self.K2_SetActorRotation` (`self.K2_GetActorRotation`)))

(event `self.ReceiveHit`
  (params (MyComp :type "PrimitiveComponent Object Reference") (Other :type "Actor Object Reference") (OtherComp :type "PrimitiveComponent Object Reference") (bSelfMoved :type Boolean) (HitLocation :type "Vector Structure") (HitNormal :type "Vector Structure") (NormalImpulse :type "Vector Structure") (Hit :type "HitResult Structure (by ref)"))
  (bind _returnvalue (`SceneComponent.K2_GetComponentLocation` (`self.CheckImpactLocation`)))
  (`KismetSystemLibrary.PrintString` "hit")
  (if (== Other (`/Game/Blueprints/Bow/BP_Bow_Master.CharacterReference` (`self.BowReference`)))
    (`self.K2_DestroyActor`)
    (else
      (`/Engine/EditorBlueprintResources/StandardMacros.DoOnce` false
        (:`Completed`
          (bind (_outhit _returnvalue_2) (`KismetSystemLibrary.SphereTraceSingle` _returnvalue (+ _returnvalue (0.0 0.0 5.0)) (`self.RadiusCheck`) "TraceTypeQuery1" :!label _label))
          (if _returnvalue_2
            (`/Game/Blueprints/Bow/BP_Bow_Master.DamageEvent` (`self.BowReference`) _outhit (`self.Damage`) true)
            (`self.K2_DestroyActor`)
            (else
              (set `self.RadiusCheck` (+ (`self.RadiusCheck`) 4.0))
              (goto _label))))))))

(fn `UserConstructionScript`
  (bind _projectilemovement (`self.ProjectileMovement`))
  (set `ProjectileMovementComponent.InitialSpeed` (`self.ProjectileSpeed`) _projectilemovement)
  (`KismetSystemLibrary.PrintString` (`KismetStringLibrary.Conv_VectorToString` (`MovementComponent.Velocity` _projectilemovement))))