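; BP_Special_Arrow_Pickup is a teleport arrow pickup that registers itself as the player character's TargetPointRef when spawned.
; It starts with collision off, activates its Niagara effect on BeginPlay, then enables collision and sets that reference after a short delay.
; Sphere overlap, when pickup is allowed and the character is below max teleport arrows, plays a sound, adds teleport ammo once and destroys the actor.
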(event `self.ReceiveBeginPlay`
  (`ActorComponent.Activate` (`self.Niagara`) false)
  (`KismetSystemLibrary.Delay` 0.5)
  (`self.SetActorEnableCollision` true)
  (bind _asbp_character (cast `/Game/Blueprints/Characters/BP_Character` (`GameplayStatics.GetPlayerCharacter` 0)))
  (bind _output_get (set `self.CharacterReference` _asbp_character))
  (set `/Game/Blueprints/Characters/BP_Character.TargetPointRef` self _output_get))

(event `self.Sphere.OnComponentBeginOverlap`
  (params (OverlappedComponent :type "PrimitiveComponent Object Reference") (OtherActor :type "Actor Object Reference") (OtherComp :type "PrimitiveComponent Object Reference") (OtherBodyIndex :type Integer) (bFromSweep :type Boolean) (SweepResult :type "HitResult Structure (by ref)"))
  (if (`self.CanPickUp`)
    (bind _asbp_character (cast `/Game/Blueprints/Characters/BP_Character` OtherActor))
    (if (< (`/Game/Blueprints/Characters/BP_Character.TeleportArrows` _asbp_character) (`/Game/Blueprints/Characters/BP_Character.MaxTeleportArrows` _asbp_character))
      (`/Engine/EditorBlueprintResources/StandardMacros.DoOnce` false
        (:`Completed`
          (`GameplayStatics.PlaySoundAtLocation` "/Game/FX/Sounds/Bow/PickUpArrow_Cue.PickUpArrow_Cue" (`SceneComponent.K2_GetComponentLocation` (`self.Pickup`)) (struct) 1.0 1.0 0.0 null null null)
          (`/Game/Blueprints/Characters/BP_Character.Add Arrows` _asbp_character 0 (`self.AmmoToAdd`))
          (`self.K2_DestroyActor`))))))

(fn `UserConstructionScript`
  (`self.SetActorEnableCollision` false))