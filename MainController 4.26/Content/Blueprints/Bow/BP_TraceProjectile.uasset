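; BP_TraceProjectile is a bow arrow actor that flies in a straight line between a given start and end location.
; BeginPlayCustom stores both points, rotates the arrow toward the end, and plays a timeline that lerps its position at a set play rate.
; Movement does not sweep for collisions, and the actor destroys itself when the timeline finishes.
; The particle system activates through MultiCastEnable after a brief delay.
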(event `MultiCastEnable`
  (`ActorComponent.Activate` (`self.ParticleSystem`) false))

(event `BeginPlayCustom`
  (params (StartLocation :type "Vector Structure") (EndLocation :type "Vector Structure"))
  (set `self.StartLocation` StartLocation)
  (set `self.EndLocation` EndLocation)
  (`|ExecutionSequence`
    (:`then_0`
      (`KismetSystemLibrary.Delay` 0.05)
      (`self.MultiCastEnable`))
    (:`then_1`
      (`SceneComponent.K2_SetWorldRotation` (`self.Arrow`) (`KismetMathLibrary.FindLookAtRotation` (`self.StartLocation`) (`self.EndLocation`)) false false)
      (`TimelineComponent.SetPlayRate` (`self.MoveToEndLocation`) (`self.PlayRate`))
      (bind (_direction _arrowshot) (`Timeline|MoveToEndLocation` :!via `PlayFromStart`)
        (:`Update`
          (`SceneComponent.K2_SetWorldLocation` (`self.Arrow`) (`KismetMathLibrary.VLerp` (`self.StartLocation`) (`self.EndLocation`) _arrowshot) false false))
        (:`Finished`
          (`self.K2_DestroyActor`))))))

(fn `UserConstructionScript`)