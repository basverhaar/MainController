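; Shootable target actor that takes point damage, shows it as combat text and tips over when its health runs out.
; Point damage to the Center component counts in full, while hits on AimTarget deal half, each feeding the DamageNumbers widget.
; Tick polls health and calls HandleDeath once depleted, where a timeline lerps AimScene's pitch from its current rotation to lay it flat.
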(event `self.ReceiveBeginPlay`
  (set `self.Health` 100.0)
  (set `self.DamageWidget` (cast `/Game/Blueprints/DamageNumbers` (`WidgetComponent.GetUserWidgetObject` (`self.CombatTextWidget`)) :!pure true)))

(event `self.ReceiveTick`
  (params (DeltaSeconds :type "Float (single-precision)"))
  (if (<= (`self.Health`) 0.0)
    (`self.Handle Death`)))

(event `self.ReceivePointDamage`
  (params (Damage :type "Float (single-precision)") (DamageType :type "DamageType Object Reference") (HitLocation :type "Vector Structure") (HitNormal :type "Vector Structure") (HitComponent :type "PrimitiveComponent Object Reference") (BoneName :type Name) (ShotFromDirection :type "Vector Structure") (InstigatedBy :type "Controller Object Reference") (DamageCauser :type "Actor Object Reference") (HitInfo :type "HitResult Structure (by ref)"))
  (bind _returnvalue (/ Damage 2.0))
  (bind _damagewidget (`self.DamageWidget`))
  (if (== HitComponent (`self.Center`))
    (set `self.Health` (- (`self.Health`) Damage))
    (`/Game/Blueprints/DamageNumbers.PlayCombatText` _damagewidget Damage)
    (elif (== HitComponent (`self.AimTarget`))
      (set `self.Health` (- (`self.Health`) _returnvalue))
      (`/Game/Blueprints/DamageNumbers.PlayCombatText` _damagewidget _returnvalue))))

(event `Handle Death`
  (bind _aimscene (`self.AimScene`))
  (bind (_relativerotation_roll _relativerotation_pitch _relativerotation_yaw) (`KismetMathLibrary.BreakRotator` (`SceneComponent.RelativeRotation` _aimscene)))
  (bind (_direction _newtrack_0) (`Timeline|GetHitTimeline`)
    (:`Update`
      (`SceneComponent.K2_SetRelativeRotation` _aimscene (`KismetMathLibrary.RLerp` (`SceneComponent.RelativeRotation` _aimscene) (`KismetMathLibrary.MakeRotator` _relativerotation_roll -90.0 _relativerotation_yaw) _newtrack_0) false false))))

(fn `UserConstructionScript`)